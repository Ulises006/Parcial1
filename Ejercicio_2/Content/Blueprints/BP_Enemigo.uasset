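; BP_Enemigo is an enemy actor that chases a target and shoots bullets once the player character is near.
; Each Tick, it smoothly rotates toward Objetivo and moves along local X at 1.2 times VelocidadPersonaje, unscaled by delta time.
; A one-second looping timer checks distance to BP_Personaje.
; Once within range, a self-looping Delay spawns BP_Bala at its transform every two seconds, without rechecking distance.
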(event `self.ReceiveBeginPlay`
  (`KismetSystemLibrary.K2_SetTimerDelegate` (delegate `ChecarDistancia`) 1.0 true))

(event `ChecarDistancia`
  (bind _returnvalue (`GameplayStatics.GetActorOfClass` "/Game/Blueprints/BP_Personaje.BP_Personaje_C"))
  (if (<= (`KismetMathLibrary.Vector_Distance` (`self.K2_GetActorLocation`) (`self.K2_GetActorLocation` _returnvalue)) 4000.0)
    (`KismetSystemLibrary.Delay` 2.0 :!label _label)
    (`|SpawnActorFromClass` "/Game/Blueprints/BP_Bala.BP_Bala_C" (`self.GetTransform`) "Undefined" "MultiplyWithRoot" null null)
    (goto _label)))

(event `self.ReceiveTick`
  (params (DeltaSeconds :type "Float (single-precision)"))
  (`self.MirarAlPersonaje`)
  (`self.K2_AddActorLocalOffset` (`KismetMathLibrary.MakeVector` (* (`self.VelocidadPersonaje`) 1.2))))

(fn `MirarAlPersonaje`
  (`self.K2_SetActorRotation` (`KismetMathLibrary.RInterpTo` (`self.K2_GetActorRotation`) (`KismetMathLibrary.FindLookAtRotation` (`self.K2_GetActorLocation`) (`self.K2_GetActorLocation` (`self.Objetivo`))) (`GameplayStatics.GetWorldDeltaSeconds`) 2.0)))

(fn `UserConstructionScript`)